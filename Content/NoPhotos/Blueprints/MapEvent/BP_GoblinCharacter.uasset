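; BP_GoblinCharacter is a goblin character for map events that plays visual effects when it spawns and despawns.
; On each spawn or despawn presentation event, it spawns two Niagara systems at the actor's location, the Demonslayer Akaza effect and its optimized variant.
; Both systems are deactivated after a two-second delay, and the Blueprint contains no other active logic.
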(event `self.BP_OnSpawnPresentationStarted`
  (bind _returnvalue (`self.K2_GetActorLocation`))
  (bind _returnvalue_2 (`NiagaraFunctionLibrary.SpawnSystemAtLocation` "/Game/NoPhotos/Blueprints/MapEvent/Demonslayer_Akaza/Niagaras/NS_Demonslayer_Akaza.NS_Demonslayer_Akaza" _returnvalue (struct :`Pitch` 90.0)))
  (bind _returnvalue_3 (`NiagaraFunctionLibrary.SpawnSystemAtLocation` "/Game/NoPhotos/Blueprints/MapEvent/Demonslayer_Akaza/Niagaras/NS_Demonslayer_Akaza_Optimized.NS_Demonslayer_Akaza_Optimized" _returnvalue (struct :`Pitch` 90.0)))
  (`KismetSystemLibrary.Delay` 2.0)
  (`ActorComponent.Deactivate` _returnvalue_2)
  (`ActorComponent.Deactivate` _returnvalue_3))

(event `self.BP_OnDespawnPresentationStarted`
  (bind _returnvalue (`self.K2_GetActorLocation`))
  (bind _returnvalue_2 (`NiagaraFunctionLibrary.SpawnSystemAtLocation` "/Game/NoPhotos/Blueprints/MapEvent/Demonslayer_Akaza/Niagaras/NS_Demonslayer_Akaza.NS_Demonslayer_Akaza" _returnvalue (struct :`Pitch` 90.0)))
  (bind _returnvalue_3 (`NiagaraFunctionLibrary.SpawnSystemAtLocation` "/Game/NoPhotos/Blueprints/MapEvent/Demonslayer_Akaza/Niagaras/NS_Demonslayer_Akaza_Optimized.NS_Demonslayer_Akaza_Optimized" _returnvalue (struct :`Pitch` 90.0)))
  (`KismetSystemLibrary.Delay` 2.0)
  (`ActorComponent.Deactivate` _returnvalue_2)
  (`ActorComponent.Deactivate` _returnvalue_3))

(fn `UserConstructionScript`)