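; BP_BuiltInCase is a breakable relic display case Blueprint that reacts to damage and breakage events.
; When damaged, it plays a glass-hit sound through the NP sound subsystem, getting louder as remaining health drops.
; When broken, it plays a glass-shatter sound at its location and prints a Korean debug string saying the case is smashed.
; The graph holds no health logic of its own, only these feedback reactions.
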(event `self.OnCaseDamaged`
  (params (RemainingHealthRatio :type "Float (single-precision)"))
  (`NPSoundSubsystem.PlaySFXAtLocation` :`self` (subsystem `NPSoundSubsystem`) :`Sound` "/Game/NoPhotos/Resources/Sound/SoundEffect/Relic/GlassHit.GlassHit" :`Volume` (+ (- 1.0 RemainingHealthRatio) 1.0) :`AttenuationSettings` null :`ConcurrencySettings` null))

(event `self.OnCaseBroken`
  ; Comment
  (`NPSoundSubsystem.PlaySFXAtLocation` :`self` (subsystem `NPSoundSubsystem`) :`Sound` "/Game/NoPhotos/Resources/Sound/SoundEffect/Relic/GlassBroken.GlassBroken" :`Location` (`self.K2_GetActorLocation`) :`AttenuationSettings` null :`ConcurrencySettings` null)
  (`KismetSystemLibrary.PrintString` "케이스 박살"))

(fn `UserConstructionScript`)