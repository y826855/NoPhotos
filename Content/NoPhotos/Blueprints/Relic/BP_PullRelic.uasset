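; BP_PullRelic is a relic actor that moves vertically each time its NPPullGimmick component reports a successful pull.
; On BeginPlay it binds to that event and caches its starting location.
; Each success replays the MoveUp timeline, offsetting Z from the cached start by curve value times current pull count times MoveHeight.
; When the timeline finishes, it notifies the gimmick that the pull is complete.
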(event `self.ReceiveBeginPlay`
  (add `NPPullGimmickComponent.OnPullSucceeded` (`self.NPPullGimmick`) (delegate `OnPullSucceeded_Event`))
  (set `self.New Relative Location` (`self.K2_GetActorLocation`)))

(event `OnPullSucceeded_Event`
  (params (CurrentPullCount :type Integer) (RequiredPullCount :type Integer))
  (set `self.Current Pull Count` CurrentPullCount)
  (bind (_direction _move) (`Timeline|MoveUp` :!via `PlayFromStart`)
    (:`Update`
      (`self.K2_SetActorRelativeLocation` (+ (`self.New Relative Location`) (`KismetMathLibrary.MakeVector` 0.0 0.0 (* _move (`self.Current Pull Count`) (`self.MoveHeight`))))))
    (:`Finished`
      (`NPPullGimmickComponent.NotifyPullFinished` (`self.NPPullGimmick`)))))

(fn `UserConstructionScript`)