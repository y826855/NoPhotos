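; B_Sun is the sun actor, which drives a noise sound according to the player's distance from it.
; It caches the player character on BeginPlay, then every Tick maps that distance through a clamped range to the volume and pitch multipliers of SunNoise, so both drop as the player moves away.
; The mapped value is also printed to screen every frame as debug output.
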(event `self.ReceiveBeginPlay`
  (set `self.Player Reference` (`GameplayStatics.GetPlayerCharacter` 0)))

(event `self.ReceiveTick`
  (params (DeltaSeconds :type "Float (single-precision)"))
  (bind _sun_noise (`self.Sun Noise`))
  (bind _returnvalue (`KismetMathLibrary.MapRangeClamped` (`KismetMathLibrary.Vector_Distance` (`self.K2_GetActorLocation` (`self.Player Reference`)) (`self.K2_GetActorLocation` self)) 1000000.0 2500000.0 1.0))
  (if (`KismetSystemLibrary.IsValid` (`self.Player Reference`))
    (`AudioComponent.SetVolumeMultiplier` _sun_noise _returnvalue)
    (`AudioComponent.SetPitchMultiplier` _sun_noise _returnvalue)
    (`KismetSystemLibrary.PrintString` (`KismetStringLibrary.Conv_DoubleToString` _returnvalue))))

(fn `UserConstructionScript`)